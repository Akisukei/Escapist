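; Openable door actor that swings open and closed when its OpenDoor component receives open or close requests.
; It stores its starting rotation at BeginPlay, then a Door_Swing timeline adds a yaw offset to that rotation each update.
; Closing plays the timeline in reverse, and an event track on the timeline plays a door lock sound at the actor's location.
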(event `self.ReceiveBeginPlay`
  ;[1 1 1] Set init rotation to BP variable
  (set `self.Initial Rotation` (`self.K2_GetActorRotation`)))

(event `self.OpenDoor.OnOpenRequest`
  (bind (_direction _opening_angle) (`Timeline|Door_Swing` :!label _label)
    (:`Update`
      (`self.K2_SetActorRotation` (`KismetMathLibrary.ComposeRotators` (`KismetMathLibrary.MakeRotator` 0.0 0.0 _opening_angle) (`self.Initial Rotation`))))
    (:`Opening Sound`
      ;[1 1 1] Play sound when open
      (`GameplayStatics.PlaySoundAtLocation` "/Game/Audio/door-lock.door-lock" (`self.K2_GetActorLocation`) (struct) 1.0 1.0 0.0 null null null))))

(event `self.OpenDoor.OnCloseRequest`
  (goto _label :!via `Reverse`))

(fn `UserConstructionScript`)